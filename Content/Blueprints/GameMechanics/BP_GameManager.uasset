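; BP_GameManager is a game manager Blueprint that tracks the mouse position and provides a restart event for the game.
; Each Tick it reads the mouse position from BP_AstraxPlayerController and stores it in MousePosition as a fraction of viewport size.
; The axes are swapped: X holds the vertical fraction and Y the horizontal.
; A separate RestartThetGame event calls RestartGame on the current GameMode.
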(event EventBeginPlay)

(event Collision|EventActorBeginOverlap
  (params (OtherActor :type Actor%20Object%20Reference)))

(event EventTick
  (params (DeltaSeconds :type Float%20%28single-precision%29))
  (bind _asbp_astrax_player_controller (Utilities|Casting|CastToBP_AstraxPlayerController (Game|GetPlayerController 0)))
  (Variables|Default|SetMousePosition (Math|Vector2D|MakeVector2D (/ (.LocationY (Game|Player|GetMousePosition _asbp_astrax_player_controller)) (Math|Conversions|ToFloat(Integer) (.SizeY (HUD|GetViewportSize _asbp_astrax_player_controller)))) (/ (.LocationX (Game|Player|GetMousePosition _asbp_astrax_player_controller)) (Math|Conversions|ToFloat(Integer) (.SizeX (HUD|GetViewportSize _asbp_astrax_player_controller)))))))

(event EventRestartThetGame
  (bind _asgame_mode (Utilities|Casting|CastToGameMode (Game|GetGameMode)))
  (Class|GameMode|RestartGame _asgame_mode))

(fn ConstructionScript)